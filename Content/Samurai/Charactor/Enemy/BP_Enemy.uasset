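; Samurai enemy character that wields a katana and detects and faces the player.
; On begin play it initializes a montage component and a damage-check component on the katana's sockets, then toggles damage tracing each tick from a flag.
; A sphere overlap with a Player-tagged actor sets the blackboard Target, after which the capsule rotates toward that actor every tick.
; Arm and try-to-arm events toggle state flags and mesh visibility.
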(event OnComponentBeginOverlap(Sphere)
  (params (OverlappedComponent :type Primitive%20Component%20Object%20Reference) (OtherActor :type Actor%20Object%20Reference) (OtherComp :type Primitive%20Component%20Object%20Reference) (OtherBodyIndex :type Integer) (bFromSweep :type Boolean) (SweepResult :type Hit%20Result%20Structure%20%28by%20ref%29))
  (Variables|Default|SetOther%20Actor OtherActor)
  (if (Actor|ActorHasTag OtherActor "Player")
    (AI|Components|Blackboard|SetValueasObject (AI|GetBlackboard self) (Utilities|Name|MakeLiteralName "Target") OtherActor)
    (Variables|Default|SetHasTarget true)))

(event Custom|TryToArmEvent
  (bind _trytoarm (Variables|Default|GetTryToArm))
  (if (Variables|Default|GetIsTryToArm)
    (Variables|Default|SetIsTryToArm false)
    (Development|SetHiddeninGame _trytoarm true false)
    (else
      (Variables|Default|SetIsTryToArm true)
      (Development|SetHiddeninGame _trytoarm false false))))

(event Custom|ArmedEvent
  (bind _target (Variables|Default|GetTarget))
  (if (Variables|Default|GetIsArmed)
    (Variables|Default|SetIsArmed false)
    (Development|SetHiddeninGame _target true false)
    (else
      (Variables|Default|SetIsArmed true)
      (Development|SetHiddeninGame _target false false))))

(event EventTick
  (params (DeltaSeconds :type Float%20%28single-precision%29))
  (bind _self self)
  (bind _other_actor (Variables|Default|GetOther%20Actor))
  (bind _bp_damagecheck (Variables|Default|GetBP_DamageCheck))
  (bind _returnvalue (Transformation|GetActorLocation _self))
  (bind _returnvalue_2 (Transformation|GetActorLocation _other_actor))
  (Utilities|FlowControl|Sequence
    (:then_0
      (if (Variables|Default|GetEnableDoDAmage)
        (Default|EnableTrace _bp_damagecheck)
        (else
          (Default|DisableTrace _bp_damagecheck))))
    (:then_1
      (if (Variables|Default|GetHasTarget)
        (Transformation|SetWorldRotation (Variables|Default|GetCapsuleComponent _self) (Math|Rotator|FindLookatRotation (Math|Vector|MakeVector (.x _returnvalue) (.y _returnvalue) 0.0) (Math|Vector|MakeVector (.x _returnvalue_2) (.y _returnvalue_2) 0.0)) false false)))))

(event EventBeginPlay
  (Default|Init (Variables|Default|GetBP_PlayAnimMontageComponent) self)
  (Default|InitWeaponSockets (Variables|Default|GetBP_DamageCheck) (Variables|Default|GetKatana)))

(fn ConstructionScript
  (|CallParentFunction))