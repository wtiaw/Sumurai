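; Actor component that runs melee weapon hit detection between Player- and Enemy-tagged characters.
; While tracing is enabled, each tick it line-traces every weapon socket from its previous location to its current one, so fast swings sweep continuously.
; Each struck character is ignored until tracing is disabled.
; Depending on character type, hits trigger a block reaction or a directional hit, with matching sound and particles.
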(event Custom|EnableTrace
  (Variables|Default|SetTraceOpen true)
  (CallFunction|UpdateSocket)
  (Utilities|FlowControl|DoOnce false
    (:Completed
      (Audio|PlaySound2D (Utilities|Array|Get(acopy) (Variables|Default|GetWosh) (Math|Random|RandomInteger (Utilities|Array|Length (Variables|Default|GetWosh)))) 1.0 1.0 0.0 0 0))))

(event Custom|DisableTrace
  (Variables|Default|SetTraceOpen false)
  (Utilities|Array|Clear (Variables|Default|GetDamagedActor))
  (Utilities|Map|Clear (Variables|Default|GetPreSocketLocation))
  (Utilities|FlowControl|DoOnce false) ; enters at Reset
)

(event Custom|InitWeaponSockets
  (params (Weapon :type Scene%20Component%20Object%20Reference))
  (Utilities|IsValid Weapon
    (:Is%20Valid
      (bind _output_get (Variables|Default|SetWeapom Weapon))
      (Variables|Default|SetSocketName (Transformation|GetAllSocketNames _output_get)))))

(event Custom|UpdateSocket
  (for _array_element (Variables|Default|GetSocketName)
    (Utilities|Map|Add (Variables|Default|GetPreSocketLocation) _array_element (Transformation|GetSocketLocation (Variables|Default|GetWeapom) _array_element))))

(event Custom|Trace
  (for _array_element (Variables|Default|GetSocketName)
    (Variables|Default|SetStart (.Value (Utilities|Map|Find (Variables|Default|GetPreSocketLocation) _array_element)))
    (Variables|Default|SetEnd (Transformation|GetSocketLocation (Variables|Default|GetWeapom) _array_element))
    (bind _outhits (Class|KismetSystemLibrary|LineTraceMultiforObjects (.Value (Utilities|Map|Find (Variables|Default|GetPreSocketLocation) _array_element)) (Transformation|GetSocketLocation (Variables|Default|GetWeapom) _array_element) (Utilities|Array|MakeArray "ObjectTypeQuery3") false (Variables|Default|GetDamagedActor) "None" true "(R=0.019574,G=1.000000,B=0.000000,A=0.000000)" "(R=1.000000,G=0.058563,B=0.000000,A=1.000000)"))
    (for _array_element_2 _outhits
      (Variables|Default|SetHitLocation (.Location (Collision|BreakHitResult _array_element_2)))
      (if (Actor|ActorHasTag (Components|GetOwner) "Player")
        (if (Actor|ActorHasTag (.HitActor (Collision|BreakHitResult _array_element_2)) "Enemy")
          (bind _asbp_base_charactor (Utilities|Casting|CastToBP_BaseCharactor (.HitActor (Collision|BreakHitResult _array_element_2)) :!label _label))
          (Variables|Default|SetBase%20Charactor _asbp_base_charactor)
          (Utilities|Array|Add (Variables|Default|GetDamagedActor) _asbp_base_charactor)
          (if (Variables|/Game/Samurai/Charactor/BaseBluePrints/BP_BaseCharactor.BP_BaseCharactor_C|GetCanBeHitted _asbp_base_charactor)
            (if (Utilities|Enum|Equal(Enum) (Variables|/Game/Samurai/Charactor/BaseBluePrints/BP_BaseCharactor.BP_BaseCharactor_C|GetCharactorType (Variables|Default|GetBase%20Charactor)) "NewEnumerator3")
              (Default|Block (Variables|/Game/Samurai/Charactor/BaseBluePrints/BP_BaseCharactor.BP_BaseCharactor_C|GetBP_PlayAnimMontageComponent (Variables|Default|GetBase%20Charactor)) (- (Variables|Default|GetStart) (Variables|Default|GetEnd)))
              (Audio|PlaySound2D "/Game/Sword_Fighting_SFX/Wavs/Sword_Hit_2.Sword_Hit_2" 1.0 1.0 0.0 0 0)
              (Effects|SpawnEmitteratLocation "/Game/CloseCombat/Effects/Impacts/P_Imp_Metal_Block.P_Imp_Metal_Block" (Variables|Default|GetHitLocation))
              (elif (Utilities|Enum|Equal(Enum) (Variables|/Game/Samurai/Charactor/BaseBluePrints/BP_BaseCharactor.BP_BaseCharactor_C|GetCharactorType (Variables|Default|GetBase%20Charactor)) "NewEnumerator2")
                (Default|Block (Variables|/Game/Samurai/Charactor/BaseBluePrints/BP_BaseCharactor.BP_BaseCharactor_C|GetBP_PlayAnimMontageComponent (Variables|Default|GetBase%20Charactor)) (- (Variables|Default|GetStart) (Variables|Default|GetEnd)))
                (Audio|PlaySound2D "/Game/Sword_Fighting_SFX/Wavs/Sword_Hit_4.Sword_Hit_4" 1.0 1.0 0.0 0 0)
                (Effects|SpawnEmitteratLocation "/Game/CloseCombat/Effects/Impacts/P_Imp_Metal_Defend.P_Imp_Metal_Defend" (Variables|Default|GetHitLocation))
                (else
                  (Default|Hit (Variables|/Game/Samurai/Charactor/BaseBluePrints/BP_BaseCharactor.BP_BaseCharactor_C|GetBP_GetHit _asbp_base_charactor) (Math|Vector|Normalize (Math|Vector|MakeVector (.x (- (Variables|Default|GetStart) (Variables|Default|GetEnd))) (.y (- (Variables|Default|GetStart) (Variables|Default|GetEnd))) 0.0) 1.0))
                  (Effects|SpawnEmitteratLocation "/Game/FXVillesBloodVFXPack/Particles/PS_Blood_Slice.PS_Blood_Slice" (Variables|Default|GetHitLocation) (Math|Conversions|RotationFromXVector (Math|Vector|RotateVector (- (Variables|Default|GetStart) (Variables|Default|GetEnd)) "0,-90.000000, 0")))
                  (Audio|PlaySound2D (Utilities|Array|Get(acopy) (Variables|Default|GetHitFlesh) (Math|Random|RandomInteger (Utilities|Array|Length (Variables|Default|GetHitFlesh)))) 1.0 1.0 0.0 0 0))))))
        (elif (Actor|ActorHasTag (Components|GetOwner) "Enemy")
          (if (Actor|ActorHasTag (.HitActor (Collision|BreakHitResult _array_element_2)) "Player")
            (goto _label)))))))

(event EventTick
  (params (DeltaSeconds :type Float%20%28single-precision%29))
  (if (Variables|Default|GetTraceOpen)
    (Utilities|FlowControl|Sequence
      (:then_0
        (CallFunction|Trace))
      (:then_1
        (CallFunction|UpdateSocket)))))