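; BP_GetHitComponent is a component that classifies an incoming hit by direction for its owning BP_BaseCharactor.
; The Hit event compares the attack direction to the owner's forward vector, using dot-product thresholds for front, back and diagonal sectors and cross-product Z for side.
; It writes the result to the character as a "Hit_"-prefixed HitDirection (F, B, FL, FR, L, R) and switches its InputType.
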(event Custom|Hit
  (params (AttackDirection :type Vector))
  (bind _returnvalue (Components|GetOwner))
  (bind _returnvalue_2 (Transformation|GetActorForwardVector _returnvalue))
  (bind _returnvalue_3 (Math|Vector|CrossProduct AttackDirection _returnvalue_2))
  (bind _returnvalue_4 (Math|Vector|DotProduct AttackDirection _returnvalue_2))
  (bind _returnvalue_5 (> (.z _returnvalue_3) 0.0))
  (bind _asbp_base_charactor (Utilities|Casting|CastToBP_BaseCharactor _returnvalue))
  (Variables|Default|SetBaseCharactor _asbp_base_charactor)
  (if (> _returnvalue_4 0.86)
    (Variables|Default|SetHitDirection "F")
    (elif (< _returnvalue_4 -0.7)
      (Variables|Default|SetHitDirection "B")
      (elif (> _returnvalue_4 0.5)
        (if _returnvalue_5
          (Variables|Default|SetHitDirection "FL")
          (else
            (Variables|Default|SetHitDirection "FR")))
        (elif _returnvalue_5
          (Variables|Default|SetHitDirection "L")
          (else
            (Variables|Default|SetHitDirection "R"))))))
  (Variables|/Game/Samurai/Charactor/BaseBluePrints/BP_BaseCharactor.BP_BaseCharactor_C|SetInputType (Variables|Default|GetBaseCharactor) "NewEnumerator4")
  (Variables|/Game/Samurai/Charactor/BaseBluePrints/BP_BaseCharactor.BP_BaseCharactor_C|SetHitDirection (Variables|Default|GetBaseCharactor) (Utilities|String|Append "Hit_" (Variables|Default|GetHitDirection))))