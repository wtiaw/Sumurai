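; BP_TypeComponent is a component for BP_Enemy owners that relays an enemy's danger cue to the player's screen.
; On BeginPlay it caches the player controller and owning enemy, then binds to the OnShowDanger dispatcher on the enemy mesh's ABP_Enemy anim instance.
; When that fires, it calls ShowImage on BP_PlayerController and UpdataImage on the controller's danger widget.
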(event Custom|Danger
  (bind _as_bp_player_controller (Variables|Default|GetAs%20BP%20Player%20Controller))
  (Default|ShowImage _as_bp_player_controller)
  (Default|UpdataImage (Variables|/Game/Samurai/Charactor/Player/Blueprints/BP_PlayerController.BP_PlayerController_C|GetAs%20WB%20Danger _as_bp_player_controller)))

(event EventBeginPlay
  (bind _asbp_player_controller (Utilities|Casting|CastToBP_PlayerController (Game|GetPlayerController 0)))
  (Variables|Default|SetAs%20BP%20Player%20Controller _asbp_player_controller)
  (bind _asbp_enemy (Utilities|Casting|CastToBP_Enemy (Components|GetOwner)))
  (bind _output_get (Variables|Default|SetAs%20BP%20Enemy _asbp_enemy))
  (bind _asabp_enemy (Utilities|Casting|CastToABP_Enemy (Components|SkeletalMesh|GetAnimInstance (Variables|/Script/Engine.Character|GetMesh _output_get))))
  (EventDispatchers|BindEventtoOnShowDanger _asabp_enemy (delegate Custom|Danger)))

(event EventTick
  (params (DeltaSeconds :type Float%20%28single-precision%29)))