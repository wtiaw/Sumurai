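; Component that plays a samurai character's attack, avoid, hit and block montages and updates its combat state.
; Tick resets state to Idle except during PowerStorage, as the montage-playing check is empty, then dispatches on InputType, with debug prints.
; Montage sections follow attack type, move axis or hit direction; Attack skips BP_Charactor.
; Block picks its section from the screen-projected attack direction and left/right stance, flipping stance on crossovers and nudging the character backward.
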(event Custom|Init
  (params (Charactor :type BP%20Base%20Charactor%20Object%20Reference))
  (bind _output_get (Variables|Default|SetCharactor Charactor))
  (Variables|Default|SetMesh (Variables|/Script/Engine.Character|GetMesh _output_get))
  (Variables|Default|SetAnimInstance (Components|SkeletalMesh|GetAnimInstance (Variables|/Script/Engine.Character|GetMesh _output_get))))

(event Custom|Avoid
  (params (Type :type CharactorType%20Enum :default "NewEnumerator0"))
  (Animation|Montage|PlayMontage (Variables|Default|GetMesh) "/Game/Samurai/Animation/AnimaltionMontage/AvoidMontage.AvoidMontage" 1.0 0.0 (Utilities|String|StringToName (Utilities|String|Append "Avoid_" (Avoid|GetAvoidDirection)))
    (:then
      (Variables|/Game/Samurai/Charactor/BaseBluePrints/BP_BaseCharactor.BP_BaseCharactor_C|SetCharactorType (Variables|Default|GetCharactor) Type))
    (:OnCompleted
      (Variables|/Game/Samurai/Charactor/BaseBluePrints/BP_BaseCharactor.BP_BaseCharactor_C|SetCharactorType (Variables|Default|GetCharactor) "NewEnumerator0"))))

(event Custom|Hit
  (params (Type :type CharactorType%20Enum :default "NewEnumerator0"))
  (bind _charactor (Variables|Default|GetCharactor))
  (Animation|Montage|PlayMontage (Variables|Default|GetMesh) "/Game/Samurai/Animation/AnimaltionMontage/HitMontage.HitMontage" 1.0 0.0 (Utilities|String|StringToName (Variables|/Game/Samurai/Charactor/BaseBluePrints/BP_BaseCharactor.BP_BaseCharactor_C|GetHitDirection (Variables|Default|GetCharactor)))
    (:then
      (Variables|/Game/Samurai/Charactor/BaseBluePrints/BP_BaseCharactor.BP_BaseCharactor_C|SetCharactorType (Variables|Default|GetCharactor) Type)
      (Variables|/Game/Samurai/Charactor/BaseBluePrints/BP_BaseCharactor.BP_BaseCharactor_C|SetInputType _charactor "NewEnumerator0"))
    (:OnBlendOut
      (Variables|/Game/Samurai/Charactor/BaseBluePrints/BP_BaseCharactor.BP_BaseCharactor_C|SetCharactorType _charactor "NewEnumerator0"))))

(event Custom|Attack
  (params (Type :type CharactorType%20Enum :default "NewEnumerator0") (AttackSection :type Name))
  (Animation|Montage|PlayMontage (Variables|Default|GetMesh) "/Game/Samurai/Animation/AnimaltionMontage/AttackMontage.AttackMontage" 1.0 0.0 AttackSection
    (:then
      (Variables|/Game/Samurai/Charactor/BaseBluePrints/BP_BaseCharactor.BP_BaseCharactor_C|SetCharactorType (Variables|Default|GetCharactor) Type))
    (:OnBlendOut
      (Variables|/Game/Samurai/Charactor/BaseBluePrints/BP_BaseCharactor.BP_BaseCharactor_C|SetCharactorType (Variables|Default|GetCharactor) "NewEnumerator0"))))

(event Custom|Block
  (params (AttackDirection :type Vector))
  (Animation|Montage|PlayMontage (Variables|Default|GetMesh) "/Game/Samurai/Animation/AnimaltionMontage/DefendMontage.DefendMontage" 1.0 0.0 (CallFunction|GetBlockDirection AttackDirection)
    (:then
      (Variables|Default|SetBack true)
      (Transformation|AddActorLocalOffset (Variables|Default|GetCharactor) "-40.000000, 0, 0" false false))))

(event EventTick
  (params (DeltaSeconds :type Float%20%28single-precision%29))
  (bind _charactor (Variables|Default|GetCharactor))
  (bind _charactor_2 (Variables|Default|GetCharactor))
  (bind _charactor_3 (Variables|Default|GetCharactor))
  (bind _returnvalue (Utilities|String|ToString(Object) _charactor))
  (Utilities|IsValid (Variables|Default|GetCharactor)
    (:Is%20Valid
      (Utilities|IsValid (Variables|Default|GetMesh)
        (:Is%20Valid
          (Utilities|FlowControl|Sequence
            (:then_0
              (bind _output_get (Variables|Default|SetEnableMove (> (Math|Vector2D|Vector2DLength (Variables|/Game/Samurai/Charactor/BaseBluePrints/BP_BaseCharactor.BP_BaseCharactor_C|GetMoveAxis (Variables|Default|GetCharactor))) 0.0)))
              (Variables|/Game/Samurai/Charactor/BaseBluePrints/BP_BaseCharactor.BP_BaseCharactor_C|SetEnableMove (Variables|Default|GetCharactor) _output_get))
            (:then_1
              (Utilities|FlowControl|Sequence
                (:then_0
                  (if (not (Utilities|GetAnimIsPlaying))
                    (if (Utilities|Enum|NotEqual(Enum) (Variables|/Game/Samurai/Charactor/BaseBluePrints/BP_BaseCharactor.BP_BaseCharactor_C|GetCharactorType _charactor_3) "NewEnumerator9")
                      (Variables|/Game/Samurai/Charactor/BaseBluePrints/BP_BaseCharactor.BP_BaseCharactor_C|SetCharactorType _charactor_3 "NewEnumerator0"))))
                (:then_1
                  (switch Utilities|FlowControl|Switch|SwitchonCharactorType (Variables|/Game/Samurai/Charactor/BaseBluePrints/BP_BaseCharactor.BP_BaseCharactor_C|GetInputType (Variables|Default|GetCharactor))
                    (:NewEnumerator1
                      (|Attack1))
                    (:NewEnumerator3
                      (Variables|/Game/Samurai/Charactor/BaseBluePrints/BP_BaseCharactor.BP_BaseCharactor_C|SetCharactorType (Variables|Default|GetCharactor) "NewEnumerator3"))
                    (:NewEnumerator2
                      (Variables|/Game/Samurai/Charactor/BaseBluePrints/BP_BaseCharactor.BP_BaseCharactor_C|SetCharactorType (Variables|Default|GetCharactor) "NewEnumerator2"))
                    (:NewEnumerator4
                      (|Hit_1))
                    (:NewEnumerator7
                      (|Avoid_2))))
                (:then_2
                  (Development|PrintString (Utilities|String|Append _returnvalue (Utilities|String|EnumtoString (Variables|/Game/Samurai/Charactor/BaseBluePrints/BP_BaseCharactor.BP_BaseCharactor_C|GetCharactorType _charactor_2))) true true "(R=0.000000,G=0.660000,B=1.000000,A=1.000000)" 0.0)
                  (Development|PrintString (Utilities|String|Append _returnvalue (Utilities|String|EnumtoString (Variables|/Game/Samurai/Charactor/BaseBluePrints/BP_BaseCharactor.BP_BaseCharactor_C|GetInputType _charactor_2))) true true "(R=1.000000,G=0.024960,B=0.000000,A=1.000000)" 0.0)
                  (if (Variables|Default|GetBack)
                    _))))))))))

(fn GetAvoidDirection
  (bind _charactor (Variables|Default|GetCharactor))
  (bind _moveaxis (Variables|/Game/Samurai/Charactor/BaseBluePrints/BP_BaseCharactor.BP_BaseCharactor_C|GetMoveAxis _charactor))
  (if (== (.x _moveaxis) -1.0)
    (Variables|Avoid|SetAvoidDirection "L")
    (elif (== (.x _moveaxis) 1.0)
      (Variables|Avoid|SetAvoidDirection "R")
      (elif (<= (.y _moveaxis) 0.0)
        (Variables|Avoid|SetAvoidDirection "B")
        (else
          (Variables|Avoid|SetAvoidDirection "F")))))
  (return (Variables|Avoid|GetAvoidDirection)))

(fn GetBlockDirection
  (params (AttackDirection :type Vector))
  (bind _returnvalue (Game|GetPlayerController 0))
  (bind _charactor (Variables|Default|GetCharactor))
  (bind (_sizex _sizey _halfsizex _halfsizey) (CallFunction|GetViewPortSize _returnvalue))
  (bind _returnvalue_2 (Transformation|GetActorLocation _charactor))
  (bind _returnvalue_3 (Transformation|GetActorForwardVector _charactor))
  (bind _screenposition (Class|GameplayStatics|ProjectWorldtoScreen _returnvalue _returnvalue_2 false))
  (bind _returnvalue_4 (* _returnvalue_3 -1.0))
  (bind (_x _y) (Math|Vector2D|BreakVector2D _screenposition))
  (bind _projection (CallFunction|GetProjectionbyNormal AttackDirection _returnvalue_4))
  (bind _returnvalue_5 (Math|Float|Clamp(Float) _y 0.0 _sizey))
  (bind _returnvalue_6 (Math|Float|Clamp(Float) _x 0.0 _sizex))
  (bind _returnvalue_7 (* _projection 5e+01))
  (bind _returnvalue_8 (+ _returnvalue_2 _returnvalue_7))
  (bind _screenposition_2 (Class|GameplayStatics|ProjectWorldtoScreen _returnvalue _returnvalue_8 false))
  (bind (_x_2 _y_2) (Math|Vector2D|BreakVector2D _screenposition_2))
  (bind _returnvalue_9 (Math|Float|Clamp(Float) _x_2 0.0 _sizex))
  (bind _returnvalue_10 (Math|Float|Clamp(Float) _y_2 0.0 _sizey))
  (bind _returnvalue_11 (- _returnvalue_9 _returnvalue_6))
  (bind _returnvalue_12 (- _returnvalue_10 _returnvalue_5))
  (bind _returnvalue_13 (> _returnvalue_11 0.0))
  (bind _returnvalue_14 (< _returnvalue_12 0.0))
  (if (Variables|/Game/Samurai/Charactor/BaseBluePrints/BP_BaseCharactor.BP_BaseCharactor_C|GetIsL (Variables|Default|GetCharactor))
    (if _returnvalue_13
      (if _returnvalue_14
        (Variables|Default|SetBlockDirection "L2R_U")
        (else
          (Variables|Default|SetBlockDirection "L2R_D")))
      (Variables|/Game/Samurai/Charactor/BaseBluePrints/BP_BaseCharactor.BP_BaseCharactor_C|SetIsL (Variables|Default|GetCharactor) false)
      (elif _returnvalue_14
        (Variables|Default|SetBlockDirection "L_U")
        (else
          (Variables|Default|SetBlockDirection "L_D"))))
    (elif _returnvalue_13
      (if _returnvalue_14
        (Variables|Default|SetBlockDirection "R_U")
        (else
          (Variables|Default|SetBlockDirection "R_D")))
      (else
        (if _returnvalue_14
          (Variables|Default|SetBlockDirection "R2L_U")
          (else
            (Variables|Default|SetBlockDirection "R2L_D")))
        (Variables|/Game/Samurai/Charactor/BaseBluePrints/BP_BaseCharactor.BP_BaseCharactor_C|SetIsL (Variables|Default|GetCharactor) true))))
  (Development|PrintString (Utilities|String|ToString(Name) (Variables|Default|GetBlockDirection)) true true "(R=0.000000,G=0.660000,B=1.000000,A=1.000000)" 1e+01)
  (return (Utilities|String|StringToName (Utilities|String|Append "Defend_" (Utilities|String|ToString(Name) (Variables|Default|GetBlockDirection))))))

(fn GetProjectionbyNormal
  (params (Vector :type Vector) (Normal :type Vector))
  (return (Math|Vector|Normalize (+ (* (* Normal (Math|Float|Absolute(Float) (Math|Vector|DotProduct (Math|Vector|Normalize Vector) (Math|Vector|Normalize Normal)))) -1.0) Vector))))

(fn GetViewPortSize
  (params (PlayerController :type Player%20Controller%20Object%20Reference))
  (bind (_sizex _sizey) (HUD|GetViewportSize PlayerController))
  (return (Math|Conversions|ToFloat(Integer) _sizex) (Math|Conversions|ToFloat(Integer) _sizey) (Math|Conversions|ToFloat(Integer) (/ _sizey 2)) (Math|Conversions|ToFloat(Integer) (/ _sizex 2))))